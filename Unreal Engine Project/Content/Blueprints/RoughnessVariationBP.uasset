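; RoughnessVariationBP is an actor that shows a roughness value on a static mesh with text labels.
; On BeginPlay it fills a label from AboveText.
; Every Tick it writes CurrentRoughness to a second label and pushes it to the scalar parameter named by Property.
; It calls CreateDynamicMaterialInstance on slot 0 each frame, and nothing in the graph changes the value itself.
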(event `self.ReceiveBeginPlay`
  (`TextRenderComponent.K2_SetText` (`self.AddingText`) (`KismetTextLibrary.Conv_StringToText` (`self.AboveText`))))

(event `self.ReceiveTick`
  (params (DeltaSeconds :type "Float (single-precision)"))
  (`TextRenderComponent.K2_SetText` (`self.PropertyText`) (`KismetTextLibrary.Conv_DoubleToText` (`self.CurrentRoughness`) "HalfToEven"))
  (bind _returnvalue (`PrimitiveComponent.CreateDynamicMaterialInstance` (`self.StaticMeshComponent`) 0 null))
  (`MaterialInstanceDynamic.SetScalarParameterValue` _returnvalue (`self.Property`) (`self.CurrentRoughness`)))

(fn `UserConstructionScript`)