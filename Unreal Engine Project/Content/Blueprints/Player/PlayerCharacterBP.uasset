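; Player character Blueprint for a side-view flipbook-sprite character that moves along world X and jumps.
; The MoveRight axis feeds movement input to CharacterMovement, and the Jump action triggers a jump.
; Each tick turns the sprite to face the sign of X velocity and picks the idle or walk flipbook from the capsule's physics velocity.
; The construction script runs the same flipbook selection.
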(event `self.ReceiveTick`
  (params (DeltaSeconds :type "Float (single-precision)"))
  (`self.TurnPlayerSprite`)
  (`self.UpdateFlipbookBySpeed`))

(event `InputAxis|MoveRight`
  (params (AxisValue :type "Float (single-precision)"))
  (`PawnMovementComponent.AddInputVector` (`self.CharacterMovement`) (* (`KismetMathLibrary.MakeVector` 1.0) AxisValue) false))

(event `InputAction|Jump`
  (params (Key :type "Key Structure"))
  (:`Pressed`
    (`self.Jump`)))

(fn `TurnPlayerSprite`
  (bind _sprite (`self.Sprite`))
  (bind _x (.x (`MovementComponent.Velocity` (`self.CharacterMovement`))))
  (if (== _x 0.0)
    _
    (elif (> _x 0.0)
      (`SceneComponent.K2_SetWorldRotation` :`self` _sprite)
      (else
        (`SceneComponent.K2_SetWorldRotation` _sprite (struct :`Yaw` 180.0) false false)))))

(fn `UpdateFlipbookBySpeed`
  (bind _idleflipbook (`self.IdleFlipbook`))
  (bind _sprite (`self.Sprite`))
  (bind _sprite_2 (`self.Sprite`))
  (bind _walkflipbook (`self.WalkFlipbook`))
  (bind _returnvalue (`PrimitiveComponent.GetPhysicsLinearVelocity` (`self.CapsuleComponent`) "None"))
  (if (== _returnvalue (0.0 0.0 0.0))
    (if (!= _idleflipbook (`PaperFlipbookComponent.GetFlipbook` _sprite))
      (`PaperFlipbookComponent.SetFlipbook` _sprite _idleflipbook))
    (elif (!= _walkflipbook (`PaperFlipbookComponent.GetFlipbook` _sprite_2))
      (`PaperFlipbookComponent.SetFlipbook` _sprite_2 _walkflipbook))))

(fn `UserConstructionScript`
  (`self.UpdateFlipbookBySpeed`))