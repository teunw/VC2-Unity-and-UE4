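; Collectible pickup actor for a Roll-a-Ball game that awards points to whatever scoring actor hits it.
; Each Tick it keeps the Cube spinning by overwriting its physics angular velocity.
; On a Hit, rather than an overlap, it looks for a PlayerScoreComponent on the other actor.
; If found, it passes its PickupComponent's Points to AddScore, prints the result and destroys itself.
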(event `self.ReceiveTick`
  (params (DeltaSeconds :type "Float (single-precision)"))
  (`PrimitiveComponent.SetPhysicsAngularVelocityInDegrees` (`self.Cube`) (45.0 45.0 45.0) false "None"))

(event `self.ReceiveHit`
  (params (MyComp :type "PrimitiveComponent Object Reference") (Other :type "Actor Object Reference") (OtherComp :type "PrimitiveComponent Object Reference") (bSelfMoved :type Boolean) (HitLocation :type "Vector Structure") (HitNormal :type "Vector Structure") (NormalImpulse :type "Vector Structure") (Hit :type "HitResult Structure (by ref)"))
  (bind _returnvalue (`self.GetComponentByClass` Other "/Game/Blueprints/RollABall/PlayerScoreComponent.PlayerScoreComponent_C"))
  (if (`KismetSystemLibrary.IsValid` _returnvalue)
    (bind _newaddition (`/Game/Blueprints/RollABall/PlayerScoreComponent.AddScore` _returnvalue (`/Game/Blueprints/RollABall/PickupComponent.Points` (`self.PickupComponent`))))
    (`KismetSystemLibrary.PrintString` (`KismetStringLibrary.Conv_IntToString` _newaddition))
    (`self.K2_DestroyActor`)))

(fn `UserConstructionScript`)