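; Key pickup Blueprint that a player collects, updating both the player's state and a linked door.
; On pickup, it casts the character's PlayerState to PlayerKeyState, sets its pickup flag to true and calls SetFull(false) on the referenced Door.
; It then prints a debug "Hello", sets a very short lifespan and destroys itself.
; BeginPlay, Tick and the construction script only call their parent versions.
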(event `self.ReceiveBeginPlay`
  (`parent.ReceiveBeginPlay`))

(event `self.ReceiveTick`
  (params (DeltaSeconds :type "Float (single-precision)"))
  (`parent.ReceiveTick` DeltaSeconds))

(event `self.OnPickup`
  (params (PlayerCharacter :type "/Game/Blueprints/Player/PlayerCharacterBP Object Reference"))
  (bind _asplayer_key_state (cast `/Game/Blueprints/Player/PlayerKeyState` (`Pawn.PlayerState` PlayerCharacter)))
  (`/Game/Blueprints/Player/PlayerKeyState.SetPickup` _asplayer_key_state true)
  (`/Game/Blueprints/Stuff/KeyDoor.SetFull` (`self.Door`) false)
  (`KismetSystemLibrary.PrintText` "Hello")
  (`self.SetLifeSpan` 0.01)
  (`self.K2_DestroyActor`))

(fn `UserConstructionScript`
  (`parent.UserConstructionScript`))