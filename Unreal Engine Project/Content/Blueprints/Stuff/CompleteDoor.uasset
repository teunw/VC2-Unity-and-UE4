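; CompleteDoor is a level-completion door actor built from Top and Middle sprite components.
; The construction script calls SetFull with StartFull, swapping both sprites between full and empty variants.
; When the player character overlaps the door it only prints "Done"; no level transition or further completion logic is present yet.
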(event `self.ReceiveActorBeginOverlap`
  (params (OtherActor :type "Actor Object Reference"))
  (bind _asplayer_character_bp (cast `/Game/Blueprints/Player/PlayerCharacterBP` OtherActor))
  (`KismetSystemLibrary.PrintText` "Done"))

(fn `SetFull`
  (params (Full :type Boolean :default true))
  (bind _top (`self.Top`))
  (bind _middle (`self.Middle`))
  (if Full
    (`PaperSpriteComponent.SetSprite` _top (`self.FullSpriteTop`))
    (`PaperSpriteComponent.SetSprite` _middle (`self.FullSpriteMiddle`))
    (else
      (`PaperSpriteComponent.SetSprite` _top (`self.EmptySpriteTop`))
      (`PaperSpriteComponent.SetSprite` _middle (`self.EmptySpriteMiddle`)))))

(fn `UserConstructionScript`
  (`self.SetFull` (`self.StartFull`)))