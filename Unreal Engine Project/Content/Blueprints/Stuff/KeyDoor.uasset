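; KeyDoor is a 2D sprite door that checks whether an overlapping player has picked up a key.
; The construction script calls SetFull, which switches the Top and Middle sprites between full and empty variants, and starts them full.
; On overlap it reads KeyPickedUp from the player's PlayerKeyState and currently only prints a placeholder message, without changing the door.
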(event `self.ReceiveActorBeginOverlap`
  (params (OtherActor :type "Actor Object Reference"))
  (bind _asplayer_character_bp (cast `/Game/Blueprints/Player/PlayerCharacterBP` OtherActor))
  (bind _asplayer_key_state (cast `/Game/Blueprints/Player/PlayerKeyState` (`Pawn.PlayerState` _asplayer_character_bp)))
  (if (`/Game/Blueprints/Player/PlayerKeyState.KeyPickedUp` _asplayer_key_state)
    (`KismetSystemLibrary.PrintText` "Hello")))

(fn `SetFull`
  (params (Full :type Boolean :default true))
  (bind _top (`self.Top`))
  (bind _middle (`self.Middle`))
  (if Full
    (`PaperSpriteComponent.SetSprite` _top (`self.FullSpriteTop`))
    (`PaperSpriteComponent.SetSprite` _middle (`self.FullSpriteMiddle`))
    (else
      (`PaperSpriteComponent.SetSprite` _top (`self.EmptySpriteTop`))
      (`PaperSpriteComponent.SetSprite` _middle (`self.EmptySpriteMiddle`)))))

(fn `UserConstructionScript`
  (`self.SetFull` true))