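; CoinTile is a Paper2D sprite tile that reacts when the player character hits it.
; The construction script applies CoinSprite, and the first player hit swaps it to AfterSprite, provided that sprite is valid.
; A later hit destroys the tile if DestroyAfter is set, using the current sprite as the state check.
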(event `self.ReceiveHit`
  (params (MyComp :type "PrimitiveComponent Object Reference") (Other :type "Actor Object Reference") (OtherComp :type "PrimitiveComponent Object Reference") (bSelfMoved :type Boolean) (HitLocation :type "Vector Structure") (HitNormal :type "Vector Structure") (NormalImpulse :type "Vector Structure") (Hit :type "HitResult Structure (by ref)"))
  (cast `/Game/Blueprints/Player/PlayerCharacterBP` Other)
  (if (`KismetSystemLibrary.IsValid` (`self.AfterSprite`))
    (if (== (`PaperSpriteComponent.GetSprite` (`self.PaperSprite`)) (`self.AfterSprite`))
      (if (`self.DestroyAfter`)
        (`self.K2_DestroyActor`))
      (else
        (`PaperSpriteComponent.SetSprite` (`self.PaperSprite`) (`self.AfterSprite`))))))

(fn `UserConstructionScript`
  (`PaperSpriteComponent.SetSprite` (`self.PaperSprite`) (`self.CoinSprite`)))