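; Tile actor that shuttles back and forth between its starting location and the location of a referenced MoveTo actor.
; Tick advances a lerp alpha scaled by TimeBetweenMoves, then UpdateWalk sets the swept position in the current direction.
; CheckLerp resets the alpha and flips MoveToNode once it passes one, reversing travel.
; The target location is re-read every update, so the endpoint follows the MoveTo actor if it moves.
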(event `self.ReceiveBeginPlay`
  (`parent.ReceiveBeginPlay`)
  (set `self.WalkFrom` (`self.K2_GetActorLocation`)))

(event `self.ReceiveTick`
  (params (DeltaSeconds :type "Float (single-precision)"))
  (`parent.ReceiveTick` DeltaSeconds)
  (set `self.Lerp` (+ (/ DeltaSeconds (`self.TimeBetweenMoves`)) (`self.Lerp`)))
  (`self.UpdateWalk`))

(fn `CheckLerp`
  (if (> (`self.Lerp`) 1.0)
    (set `self.Lerp` 0.0)
    (set `self.MoveToNode` (not (`self.MoveToNode`)))))

(fn `GetCurrentLerp`
  (returns (Lerp :type "Float (double-precision)"))
  (return (/ (`self.Lerp`) (`self.TimeBetweenMoves`))))

(fn `GetNodeLocation`
  (returns (NodeLocation :type "Vector Structure"))
  (return (`self.K2_GetActorLocation` (`self.MoveTo`))))

(fn `UpdateWalk`
  (bind _nodelocation (`self.GetNodeLocation`))
  (if (`self.MoveToNode`)
    (`self.K2_SetActorLocation` (`KismetMathLibrary.VLerp` (`self.WalkFrom`) _nodelocation (`self.Lerp`)) true)
    (else
      (`self.K2_SetActorLocation` (`KismetMathLibrary.VLerp` _nodelocation (`self.WalkFrom`) (`self.Lerp`)) true)))
  (`self.CheckLerp`))

(fn `UserConstructionScript`
  (`parent.UserConstructionScript`))